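; Aura's Arcane Shards gameplay ability, which erupts a timed series of damaging shards around the point under the mouse.
; Activation places a magic circle, commits cost and plays a montage, whose event spawns BP_PointsCollection for randomly rotated ground points.
; A looping timer applies radial damage with overridden knockback and fires a GameplayCue at each point.
; After a level-scaled count, it hides the circle, commits cooldown and ends.
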(event `self.K2_ActivateAbility`
  (bind (_asynctaskproxy _datahandle) (`TargetDataUnderMouse.CreateTargetDataUnderMouse`)
    (:`ValidData`
      (bind _output_get (set `self.HitLocation` (`.Location` (`GameplayStatics.BreakHitResult` (`AbilitySystemBlueprintLibrary.GetHitResultFromTargetData` _datahandle)))))
      (message `CombatInterface.UpdateFacingTarget` (`self.GetAvatarActorFromActorInfo`) _output_get)
      (`self.ShowMagicCircle` null)
      (`MagicCircle.SetupLocation` (`self.MagicCircle`) (`self.HitLocation`))
      (`self.K2_CommitAbilityCost` false)
      (`AbilityTask_PlayMontageAndWait.CreatePlayMontageAndWaitProxy` "None" "/Game/Assets/Characters/Aura/Animations/Abilities/AM_ArcaneShards.AM_ArcaneShards"
        (:`then`
          (`AbilityTask_WaitGameplayEvent.WaitGameplayEvent` (struct :`TagName` "Event.Montage.ArcaneShader") null
            (:`EventReceived`
              ; 产生Shader位置，然后适当修改他们的位置
              (bind _returnvalue (`|SpawnActorFromClass` "/Game/Blueprints/AbilitySystem/Aura/Abilities/Arcane/ArcaneShaders/BP_PointsCollection.BP_PointsCollection_C" (`KismetMathLibrary.Conv_VectorToTransform` (`self.HitLocation`)) "AlwaysSpawn" "MultiplyWithRoot" null null))
              (set `self.Count` 0)
              (set `self.Points` (`PointCollectionActor.GetGroundPoints` _returnvalue (`self.HitLocation`) (`self.NumPoints`) (`KismetMathLibrary.RandomFloatInRange` 0.0 360.0)))
              (bind _returnvalue_2 (`KismetSystemLibrary.K2_SetTimerDelegate` (delegate `SpawnShaders`) (`self.SpawnDeltaTime`) true))
              (set `self.TimerHandle` _returnvalue_2))))))))

(event `SpawnShaders`
  (if (< (`self.Count`) (+ (`self.GetAbilityLevel`) (`self.NumsToSpell`)))
    (`self.SpawnShardAndCauseDamage`)
    (else
      (`KismetSystemLibrary.K2_ClearAndInvalidateTimerHandle` (`self.TimerHandle`))
      (`self.HideMagicCircle`)
      (`self.K2_CommitAbilityCooldown` false)
      (`self.K2_EndAbility`))))

(fn `SpawnShardAndCauseDamage`
  (bind _returnvalue (`self.GetAvatarActorFromActorInfo`))
  ; 获得shard的生成位置
  (set `self.PointLocation` (`SceneComponent.K2_GetComponentLocation` (`|GetArrayItem` (`self.Points`) (`self.Count`))))
  ; 造成伤害
  (bind _outoverlappingactor (`AuraAbilitySystemLibrary.GetLiversWithinRadius` _returnvalue (`|MakeArray` _returnvalue) (`self.RadialDamageOuterRadius`) (`self.PointLocation`)))
  (bind _output_get (set `self.TargetActors` _outoverlappingactor))
  (for _array_element _output_get
    (`AuraAbilitySystemLibrary.ApplyDamageEffect` (`self.MakeDamageAbilityEffectParams` _array_element (`self.PointLocation`) true (0.0 0.0 1.0) false (0.0 0.0 0.0) true 0.0)))
  ; 生成Shard
  (`/Engine/EditorBlueprintResources/StandardMacros.IncrementInt` (`self.Count`)
    (:`  `
      (`self.K2_ExecuteGameplayCueWithParams` (struct :`TagName` "GameplayCue.ArcaneShader") (`AbilitySystemBlueprintLibrary.MakeGameplayCueParameters` 0.0 0.0 (struct) (struct) (struct) (struct) (struct) (`self.PointLocation`))))))