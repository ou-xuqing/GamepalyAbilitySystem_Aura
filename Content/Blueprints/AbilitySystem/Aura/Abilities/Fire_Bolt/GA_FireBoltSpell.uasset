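; Gameplay ability for Aura's Fire Bolt spell, which fires projectiles toward the target under the mouse cursor.
; After committing, it stores the hit actor and location from a target data task and turns the avatar to face that point.
; The cast montage's Event.Montage.FireBolt event times SpawnProjectiles, which receives the target and a pitch override.
; The ability ends when the montage completes, blends out, is interrupted or is cancelled.
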(event `self.K2_ActivateAbility`
  ; 检查cost和cooldown，成功返回true，失败直接结束能力，cost和cooldown可以和等级相关
  (`self.K2_CommitAbility`)
  ; 获得鼠标碰撞的结果，TDUM是C++中创建的函数
  (bind (_asynctaskproxy _datahandle) (`TargetDataUnderMouse.CreateTargetDataUnderMouse`)
    (:`ValidData`
      (bind (_bblockinghit _binitialoverlap _time _distance _location _impactpoint _normal _impactnormal _physmat _hitactor) (`GameplayStatics.BreakHitResult` (`AbilitySystemBlueprintLibrary.GetHitResultFromTargetData` _datahandle)))
      (set `self.Target` _hitactor)
      (set `self.TargetLocation` _location)
      ; 调用BP_CharacterAura中的函数来修改朝向
      (message `CombatInterface.UpdateFacingTarget` (`self.GetAvatarActorFromActorInfo`) (`self.TargetLocation`))
      (`AbilityTask_PlayMontageAndWait.CreatePlayMontageAndWaitProxy` "None" "/Game/Assets/Characters/Aura/Animations/Abilities/AM_Cast_FireBolt.AM_Cast_FireBolt" 1.0 "None" false
        (:`then`
          ; 释放火球动画播到一定时间点时，生成火球。
          (`AbilityTask_WaitGameplayEvent.WaitGameplayEvent` (struct :`TagName` "Event.Montage.FireBolt") null
            (:`EventReceived`
              (`self.SpawnProjectiles` (`self.TargetLocation`) (`self.Socket Tag`) true 15.0 (`self.Target`)))))
        (:`OnCompleted`
          (`self.K2_EndAbility` :!label _label))
        (:`OnBlendOut`
          (goto _label))
        (:`OnInterrupted`
          (goto _label))
        (:`OnCancelled`
          (goto _label))))))