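; GA_Electrocute is a channeled lightning ability that fires a chaining shock beam at the target under the mouse.
; A montage gameplay event spawns the beam as ShockLoop cues on primary and additional targets, then starts a looping damage-and-cost timer.
; Input release, padded to a minimum spell time on authority, or primary target death ends it.
; Cleanup removes cues, applies damage effects server-side for deferred debuffs, and commits cooldown.
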(event `self.K2_ActivateAbility`
  (if (`KismetSystemLibrary.DoesImplementInterface` (`self.GetAvatarActorFromActorInfo`) "/Script/Aura.CombatInterface")
    ; 获得并存储鼠标命中数据，因为后面需要用
    (bind (_asynctaskproxy _datahandle) (`TargetDataUnderMouse.CreateTargetDataUnderMouse`)
      (:`ValidData`
        (`self.StoreMouseDataInfo` (`AbilitySystemBlueprintLibrary.GetHitResultFromTargetData` _datahandle))
        (`self.StoreOwnerVariables`)
        (`|ExecutionSequence`
          (:`then_0`
            (set `PlayerController.bShowMouseCursor` false (`self.OwnerController`))
            ; 在montage中播放释放技能是为了能够触发Tagevent事件，在适当时间生成光线，之后通过设置shock来播放循环动画
            ;; 当montag的混合速度过快时，无法motionwraping，因为motionwraping的时间被前面的动画占用了
            (message `CombatInterface.UpdateFacingTarget` (`self.GetAvatarActorFromActorInfo`) (`self.HitLocation`))
            (`self.K2_ExecuteGameplayCue` (struct :`TagName` "GameplayCue.ShockBrust"))
            (`AbilityTask_PlayMontageAndWait.CreatePlayMontageAndWaitProxy` "None" (`self.Montage_Electrocute`) 1.0 "None" false
              (:`then`
                (`AbilityTask_WaitGameplayEvent.WaitGameplayEvent` (struct :`TagName` "Event.Montage.Electrocute") null
                  (:`EventReceived`
                    (message `CombatInterface.SetInShockLoop` (`self.GetAvatarActorFromActorInfo`) true)
                    (`CharacterMovementComponent.DisableMovement` (`Character.CharacterMovement` (`self.OwnerCharacter`)))
                    (`self.SpawnBeam`)
                    (bind _returnvalue (`KismetSystemLibrary.K2_SetTimerDelegate` (delegate `DamageAndCost`) (`self.DamageDeltaTime`) true))
                    (set `self.DamageAndCostTimer` _returnvalue))))))
          (:`then_1`
            ; 当按住右键时间比最短施法时间要短时，延迟结束能力（为了让声音和montage和cue同步,because when activeAbility then palySound but at that time cue dont play）
            (bind (_asynctaskproxy_2 _timeheld) (`AbilityTask_WaitInputRelease.WaitInputRelease` false)
              (:`OnRelease`
                ;; 还有一种解决方案就是短按什么都不做，不过个人认为需要修改大量的蓝图节点
                (bind _output_get (set `self.Time Held` _timeheld))
                (if (> _output_get (`self.MinSpellTime`))
                  (`self.ClearTimerAndAbility` :!label _label)
                  (else
                    (`self.K2_HasAuthority`
                      (:`True`
                        (`KismetSystemLibrary.Delay` (- (`self.MinSpellTime`) (`self.Time Held`)))
                        (goto _label))
                      (:`False`
                        (`self.PrepareToEndAbility`)))))))))))))

(event `DamageAndCost`
  (`self.K2_CommitAbilityCost` false)
  (if true
    ; 不在这添加Debuff，因为怪物的受击效果和这个技能的debuff冲突了，根本都是禁止移动.When Ability Release,Caulate Debuff
    (if (`self.bFirstTraceEnemy`)
      (`self.ApplyDamage` (`self.HitActor`)))
    (else
      (`self.ClearTimerAndAbility`))))

(event `self.PrimaryTargetDeaded`
  (params (DeadActor :type "Actor Object Reference"))
  (`GameplayCueFunctionLibrary.RemoveGameplayCueOnActor` DeadActor (struct :`TagName` "GameplayCue.ShockLoop") (`self.FirstTraceTargetCueParam`))
  (`self.ClearTimerAndAbility`))

(event `self.AdditionalTargetDeaded`
  (params (DeadActor :type "Actor Object Reference"))
  (bind _additionaltargettocues (`self.AdditionalTargetToCues`))
  (bind (_value _returnvalue) (`BlueprintMapLibrary.Map_Find` _additionaltargettocues (`self.AdditionalDeadActor`)))
  ; 将传入的变量存储起来，不存可能有bug（后面还未执行到但是变量已经改变）
  (set `self.AdditionalDeadActor` DeadActor)
  (if _returnvalue
    (`GameplayCueFunctionLibrary.RemoveGameplayCueOnActor` (`self.AdditionalDeadActor`) (struct :`TagName` "GameplayCue.ShockLoop") _value)
    (`BlueprintMapLibrary.Map_Remove` _additionaltargettocues (`self.AdditionalDeadActor`))))

(fn `AddShockLoopCueToAdditionalTarget`
  (params (AdditionalTarget :type "Actor Object Reference"))
  (locals (Target :type "Actor Object Reference"))
  (bind _target (`local.Target`))
  (bind _returnvalue (`AbilitySystemBlueprintLibrary.MakeGameplayCueParameters` 0.0 0.0 (struct) (struct) (struct) (struct) (struct) (`Actor.K2_GetActorLocation` _target) (0.0 0.0 0.0) null null _target null 1 1 (`Actor.RootComponent` (`self.HitActor`))))
  (bind _output_get (set `local.Target` AdditionalTarget))
  (`BlueprintMapLibrary.Map_Add` (`self.AdditionalTargetToCues`) _output_get _returnvalue)
  (`GameplayCueFunctionLibrary.AddGameplayCueOnActor` (`local.Target`) (struct :`TagName` "GameplayCue.ShockLoop") _returnvalue))

(fn `ApplyDamage`
  (params (DamageTarget :type "Actor Object Reference"))
  (locals (DamageActor :type "Actor Object Reference"))
  (`self.ApplySingleActorDamage` DamageTarget)
  (for _array_element (`self.AdditionalTargets`)
    (`self.ApplySingleActorDamage` _array_element)))

(fn `ApplySingleActorDamage`
  (params (DamageActor :type "Actor Object Reference"))
  (bind _returnvalue (`AbilitySystemBlueprintLibrary.GetAbilitySystemComponent` (`self.GetAvatarActorFromActorInfo`)))
  (bind _returnvalue_2 (`self.GetDamageAtLevel`))
  (bind _returnvalue_3 (`AbilitySystemBlueprintLibrary.AssignTagSetByCallerMagnitude` (`AbilitySystemComponent.MakeOutgoingSpec` _returnvalue (`self.DamageEffectClass`) (`KismetMathLibrary.Conv_IntToDouble` (`self.GetAbilityLevel`)) (`AbilitySystemComponent.MakeEffectContext` _returnvalue)) (struct :`TagName` "Damage.Lightning") _returnvalue_2))
  (`AbilitySystemComponent.BP_ApplyGameplayEffectSpecToSelf` (`AbilitySystemBlueprintLibrary.GetAbilitySystemComponent` DamageActor) _returnvalue_3))

(fn `ClearTimerAndAbility`
  (`KismetSystemLibrary.K2_ClearAndInvalidateTimerHandle` (`self.DamageAndCostTimer`))
  (`self.PrepareToEndAbility`)
  (`self.K2_EndAbility`))

(fn `PrepareToEndAbility`
  (bind _hitactor (`self.HitActor`))
  (set `PlayerController.bShowMouseCursor` true (`self.OwnerController`))
  (message `CombatInterface.SetInShockLoop` (`self.GetAvatarActorFromActorInfo`) false)
  (`CharacterMovementComponent.SetMovementMode` (`Character.CharacterMovement` (`self.OwnerCharacter`)) "MOVE_Walking" 0)
  (`self.bFirstTraceEnemy`
    (:`then`
      ; 移除敌人或自己身上的gc，计算debuff是否启动，敌人眩晕，禁止移动
      (`GameplayCueFunctionLibrary.RemoveGameplayCueOnActor` (`self.HitActor`) (struct :`TagName` "GameplayCue.ShockLoop") (`self.FirstTraceTargetCueParam`))
      (message `CombatInterface.SetBeingShocked` _hitactor false)
      (`self.K2_HasAuthority`
        (:`True`
          (`AuraAbilitySystemLibrary.ApplyDamageEffect` (`self.MakeDamageAbilityEffectParams` _hitactor)))
        (:`False`
          _))
      (`self.RemoveAdditionalTargetCue`))
    (:`else`
      (`GameplayCueFunctionLibrary.RemoveGameplayCueOnActor` (`self.GetAvatarActorFromActorInfo`) (struct :`TagName` "GameplayCue.ShockLoop") (`self.FirstTraceTargetCueParam`))))
  (`self.K2_CommitAbilityCooldown` false))

(fn `RemoveAdditionalTargetCue`
  (for _array_element (`self.AdditionalTargets`)
    (bind (_value _returnvalue) (`BlueprintMapLibrary.Map_Find` (`self.AdditionalTargetToCues`) _array_element))
    (if _returnvalue
      (`GameplayCueFunctionLibrary.RemoveGameplayCueOnActor` _array_element (struct :`TagName` "GameplayCue.ShockLoop") _value)
      (message `CombatInterface.SetBeingShocked` _array_element false)
      (`self.K2_HasAuthority`
        (:`True`
          (`AuraAbilitySystemLibrary.ApplyDamageEffect` (`self.MakeDamageAbilityEffectParams` _array_element)))))))

(fn `SpawnBeam`
  (`self.TraceFirstTarget` (`self.HitLocation`))
  (bind _returnvalue (message `CombatInterface.GetWeapon` (`self.GetAvatarActorFromActorInfo`)))
  (set `self.Weapon` _returnvalue)
  (set `self.FirstTraceTargetCueParam` (`AbilitySystemBlueprintLibrary.MakeGameplayCueParameters` 0.0 0.0 (struct) (struct) (struct) (struct) (struct) (`self.HitLocation`) (0.0 0.0 0.0) null null (`self.HitActor`) null 1 1 (`self.Weapon`)))
  (bind _output_get (set `self.bFirstTraceEnemy` (`KismetSystemLibrary.DoesImplementInterface` (`self.HitActor`) "/Script/Aura.CombatInterface")))
  (if _output_get
    ; 目标是敌人，在敌人身上添加gc
    (`GameplayCueFunctionLibrary.AddGameplayCueOnActor` (`self.HitActor`) (struct :`TagName` "GameplayCue.ShockLoop") (`self.FirstTraceTargetCueParam`))
    (message `CombatInterface.SetBeingShocked` (`self.HitActor`) true)
    (bind _additionaltarget (`self.StoreAdditionalTarget`))
    (bind _output_get_2 (set `self.AdditionalTargets` _additionaltarget))
    (for _array_element _output_get_2
      (`self.AddShockLoopCueToAdditionalTarget` _array_element)
      (message `CombatInterface.SetBeingShocked` _array_element true))
    (else
      ; 目标是地板等，在自己身上添加gc
      (`GameplayCueFunctionLibrary.AddGameplayCueOnActor` (`self.GetAvatarActorFromActorInfo`) (struct :`TagName` "GameplayCue.ShockLoop") (`self.FirstTraceTargetCueParam`)))))