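; Fireball projectile for the FireBlast ability that flies outward, then either homes on a target or returns to its caster to explode.
; On the server, a timeline lerps it forward to a maximum distance, then calls FindNearestActorAndHoming.
; If that returns false, a second timeline lerps it toward the SpellActor's live location.
; Within a minimum distance, it calls OnHit and FindNearActorAndExplosionDamage, then destroys itself.
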(event `self.StartOutGoingTimeline`
  (`/Engine/EditorBlueprintResources/ActorMacros.Switch Has Authority`
    (:`Authority`
      (set `self.InitialLocation` (`self.K2_GetActorLocation`))
      (set `self.MaxLocation` (+ (`self.InitialLocation`) (* (`self.GetActorForwardVector`) (`self.MaxDistacne`))))
      (bind (_direction _outgoing) (`Timeline|StartOutGoing`)
        (:`Update`
          (`self.K2_SetActorLocation` (`KismetMathLibrary.VLerp` (`self.InitialLocation`) (`self.MaxLocation`) _outgoing)))
        (:`Finished`
          (bind _returnvalue (`self.FindNearestActorAndHoming`))
          (if (not _returnvalue)
            ; 第一阶段发散，第二阶段回收然后爆炸（爆炸造成伤害未实现）
            (bind (_direction_2 _comback) (`Timeline|CombackTimeline`)
              (:`Update`
                (`self.K2_SetActorLocation` (`KismetMathLibrary.VLerp` (`self.MaxLocation`) (`self.K2_GetActorLocation` (`self.SpellActor`)) _comback))
                (if (< (`KismetMathLibrary.VSize` (- (`self.K2_GetActorLocation`) (`self.K2_GetActorLocation` (`self.SpellActor`)))) (`self.MinDistance`))
                  (`self.OnHit`)
                  (`self.FindNearActorAndExplosionDamage`)
                  (`self.K2_DestroyActor`))))))))))

(event `self.ReceiveBeginPlay`)

(fn `UserConstructionScript`)