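; GA_ListenForEvent is a passive gameplay ability that turns incoming Attributes gameplay events into attribute effects on its owner.
; On activation it waits for any event under the Attributes tag.
; Each event builds an EventBasedEffectClass spec, sets the SetByCaller magnitude of the matching EventTags entry to the event's magnitude, zeroes the others to avoid missing-magnitude errors, then applies it to self.
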(event `self.K2_ActivateAbility`
  (bind _returnvalue (`self.GetAbilitySystemComponentFromActorInfo`))
  ; 持续的被动能力，监听event事件的发生，通过tag来分辨要干什么，然后设置相应的GE参数
  (bind (_asynctaskproxy _payload) (`AbilityTask_WaitGameplayEvent.WaitGameplayEvent` (struct :`TagName` "Attributes") null false false)
    (:`EventReceived`
      (bind (_eventtag _instigator _target _optionalobject _optionalobject2 _contexthandle _instigatortags _targettags _eventmagnitude) (break `GameplayEventData` _payload))
      (set `self.EventTag` _eventtag)
      (set `self.Event Magnitude` _eventmagnitude)
      ;; 解决SetbyMagnitude报错问题，即将其他的置0.C++中直接设置取不到数据发送错误为fasle即可
      (set `self.Spec` (`AbilitySystemComponent.MakeOutgoingSpec` _returnvalue (`self.EventBasedEffectClass`) 1.0 (`AbilitySystemComponent.MakeEffectContext` _returnvalue)))
      (for _array_element (`self.EventTags`)
        (if (`BlueprintGameplayTagLibrary.MatchesTag` _array_element (`self.EventTag`) true)
          (`AbilitySystemBlueprintLibrary.AssignTagSetByCallerMagnitude` (`self.Spec`) (`self.EventTag`) (`self.Event Magnitude`))
          (else
            (`AbilitySystemBlueprintLibrary.AssignTagSetByCallerMagnitude` (`self.Spec`) _array_element))))
      (`AbilitySystemComponent.BP_ApplyGameplayEffectSpecToSelf` (`self.GetAbilitySystemComponentFromActorInfo`) (`self.Spec`)))))