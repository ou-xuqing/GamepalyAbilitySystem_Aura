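; Enemy summon ability, using the Shaman summon montage, that spawns random minions around the battlefield.
; On activation it turns toward the combat target, shuffles the spawn locations and plays a ground Niagara effect at each.
; A montage gameplay event starts a delayed loop that spawns one AI-controlled minion per location, facing away from the summoner.
; Each spawn raises the summoner's minion count, and each minion's destruction lowers it.
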(event `self.K2_ActivateAbility`
  (bind _returnvalue (`self.GetAvatarActorFromActorInfo`))
  (bind _returnvalue_2 (+ (`|GetArrayItem` (`self.SpawnLoactions`) (`self.SpawnLocationsIndex`)) (0.0 0.0 60.0)))
  (bind _returnvalue_3 (message `AuraEnemyInterface.GetCombatTarget` _returnvalue))
  (message `CombatInterface.UpdateFacingTarget` _returnvalue (`Actor.K2_GetActorLocation` _returnvalue_3))
  (bind _returnvalue_4 (`self.GetSpawnLocations`))
  (bind _output_get (set `self.SpawnLoactions` _returnvalue_4))
  (`KismetArrayLibrary.Array_Shuffle` _output_get)
  (for _array_element _output_get
    (`NiagaraFunctionLibrary.SpawnSystemAtLocation` "/Game/Assets/Effects/Combat/NS_GroundSummon.NS_GroundSummon" _array_element))
  (`AbilityTask_PlayMontageAndWait.CreatePlayMontageAndWaitProxy` "None" "/Game/Assets/Enemies/Shaman/Animations/AM_Summon_Shaman.AM_Summon_Shaman"
    (:`then`
      (`AbilityTask_WaitGameplayEvent.WaitGameplayEvent` (struct :`TagName` "Montage.Attack.1") null
        (:`EventReceived`
          (if (< (`self.SpawnLocationsIndex`) (`KismetArrayLibrary.Array_Length` (`self.SpawnLoactions`))) :!label _label
            (message `CombatInterface.IncreaseMinionCount` (`self.GetAvatarActorFromActorInfo`) 1)
            (bind _returnvalue_5 (`|SpawnActorFromClass` (`self.GetRandomMinionClass`) (`KismetMathLibrary.MakeTransform` _returnvalue_2 (`KismetMathLibrary.FindLookAtRotation` (`Actor.K2_GetActorLocation` (`self.GetAvatarActorFromActorInfo`)) _returnvalue_2)) "AlwaysSpawn" "MultiplyWithRoot" null null))
            (add `Actor.OnDestroyed` _returnvalue_5 (delegate `OnDestroyed_Event`))
            (`Pawn.SpawnDefaultController` _returnvalue_5)
            (`/Engine/EditorBlueprintResources/StandardMacros.IncrementInt` (`self.SpawnLocationsIndex`)
              (:`  `
                (`KismetSystemLibrary.Delay` 0.2)
                (goto _label)))))))))

(event `OnDestroyed_Event`
  (params (DestroyedActor :type "Actor Object Reference"))
  (message `CombatInterface.IncreaseMinionCount` (`self.GetAvatarActorFromActorInfo`) -1))