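; BP_SlingShotRock is the rock actor for an enemy slingshot ability, adding a randomized tumbling spin to its mesh.
; BeginPlay picks random pitch, yaw and roll rates, each able to spin in either direction.
; Tick scales those rates by delta time and applies them as local rotation to RockMesh, keeping the spin frame-rate independent.
; The Blueprint's own graphs contain no movement or hit logic.
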(event `self.ReceiveBeginPlay`
  (bind _returnvalue (`KismetMathLibrary.RandomFloatInRange` -360.0 360.0))
  (set `self.PitchRotation` _returnvalue)
  (set `self.YawRotation` _returnvalue)
  (set `self.RollRotation` _returnvalue))

(event `self.ReceiveTick`
  (params (DeltaSeconds :type "Float (single-precision)"))
  (`SceneComponent.K2_AddLocalRotation` (`self.RockMesh`) (`KismetMathLibrary.MakeRotator` (* DeltaSeconds (`self.RollRotation`)) (* DeltaSeconds (`self.PitchRotation`)) (* DeltaSeconds (`self.YawRotation`))) false false))

(fn `UserConstructionScript`)