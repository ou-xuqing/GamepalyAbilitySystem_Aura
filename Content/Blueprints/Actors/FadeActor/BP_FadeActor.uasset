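; Fadeable mesh actor that turns faded and ignores a custom trace channel, with Fadein and FadeOut events meant to be called from the Character.
; Construction caches original materials and builds dynamic instances from FadeMaterials.
; Fadein applies those instances while a timeline drives their Fade scalar toward 0; FadeOut reverses it.
; On finish, Fade 1 restores materials and blocking, while 0 sets ignore, optionally including Visibility.
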(event `self.ReceiveBeginPlay`)

(event `/Game/Blueprints/Actors/FadeActor/BI_FadeInterface.FadeIn`
  ; 要在运行中替换材质，需要将材质动态实例化。fadein：替换材质后将fade从1变成0。fadeout：将fade从0变成1然后替换材质
  ;; Character中调用
  (`self.SetMaterialToDynamicInstance`)
  (bind (_direction _fade) (`Timeline|FadeTimeline` :!label _label)
    (:`Update`
      (for _array_element (`self.DynamicMaterialInstance`)
        (`MaterialInstanceDynamic.SetScalarParameterValue` _array_element "Fade" _fade)))
    (:`Finished`
      (`self.FadeFinshied` _fade))))

(event `/Game/Blueprints/Actors/FadeActor/BI_FadeInterface.FadeOut`
  ; 要在运行中替换材质，需要将材质动态实例化。fadein：替换材质后将fade从1变成0。fadeout：将fade从0变成1然后替换材质
  ;; Character中调用
  (goto _label :!via `Reverse`))

(fn `FadeFinshied`
  (params (Fade :type "Float (single-precision)"))
  (if (>= Fade 1.0)
    (`self.ReSetMaterial`)
    (`PrimitiveComponent.SetCollisionResponseToChannel` (`self.Mesh`) "ECC_GameTraceChannel2" "ECR_Block")
    (if (`self.bBlockVisibility`)
      (`PrimitiveComponent.SetCollisionResponseToChannel` (`self.Mesh`) "ECC_Visibility" "ECR_Block"))
    (elif (<= Fade 0.0)
      (`PrimitiveComponent.SetCollisionResponseToChannel` (`self.Mesh`) "ECC_GameTraceChannel2" "ECR_Ignore")
      (if (`self.bBlockVisibility`)
        (`PrimitiveComponent.SetCollisionResponseToChannel` (`self.Mesh`) "ECC_Visibility" "ECR_Ignore")))))

(fn `ReSetMaterial`
  (for (_array_element _array_index) (`self.OriginalMaterials`)
    (`PrimitiveComponent.SetMaterial` (`self.Mesh`) _array_index _array_element)))

(fn `SetMaterialToDynamicInstance`
  (for (_array_element _array_index) (`self.DynamicMaterialInstance`)
    (`PrimitiveComponent.SetMaterial` (`self.Mesh`) _array_index _array_element)))

(fn `UserConstructionScript`
  (`KismetArrayLibrary.Array_Clear` (`self.DynamicMaterialInstance`))
  (set `self.OriginalMaterials` (`MeshComponent.GetMaterials` (`self.Mesh`)))
  (for _array_element (`self.FadeMaterials`)
    (bind _returnvalue (`KismetMaterialLibrary.CreateDynamicMaterialInstance` _array_element))
    (`KismetArrayLibrary.Array_AddUnique` (`self.DynamicMaterialInstance`) _returnvalue)))