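; Base actor for moving pickups that plays an intro movement on spawn, then hands over to sine movement and rotation.
; A BeginPlay timeline drives scale and a vertical offset from the initial location, playing a sound once when the offset curve dips below zero.
; When it finishes, it calls StartSinMovement and StartRotator, which are defined outside these graphs.
; Tick applies the calculated location and rotation every frame.
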(event `self.ReceiveBeginPlay`
  (bind _big_to_small (`self.Big to Small`))
  (bind (_direction _uptodown _bigtosmall) (`Timeline|PickUpMovementTimelIne`)
    (:`Update`
      (set `self.Up to Down` _uptodown)
      (set `self.Big to Small` _bigtosmall)
      (set `self.CalculateLocation` (`self.MakeUTDLocation` (`self.Up to Down`)))
      (`self.SetActorScale3D` (`KismetMathLibrary.MakeVector` _big_to_small _big_to_small _big_to_small))
      (if (< (`self.Up to Down`) -0.1)
        (`/Engine/EditorBlueprintResources/StandardMacros.DoOnce` false
          (:`Completed`
            (`GameplayStatics.PlaySoundAtLocation` (`self.PoitionSound`) (`self.K2_GetActorLocation`) (struct) 1.0 1.0 0.0 null null null null)))))
    (:`Finished`
      (`self.StartSinMovement`)
      (`self.StartRotator`))))

(event `self.ReceiveTick`
  (params (DeltaSeconds :type "Float (single-precision)"))
  (`self.K2_SetActorLocation` (`self.CalculateLocation`))
  (`self.K2_SetActorRotation` (`self.CalculateRotation`)))

(fn `MakeUTDLocation`
  (params (A :type "Float (double-precision)"))
  (returns (ReturnValue :type "Vector Structure"))
  (return (`KismetMathLibrary.MakeVector` (.x (`self.InitialLocation`)) (.y (`self.InitialLocation`)) (+ (* A (`self.FlowMagnitude`)) (.z (`self.InitialLocation`))))))

(fn `UserConstructionScript`)