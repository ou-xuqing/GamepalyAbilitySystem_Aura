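; Enemy ranged attack ability that turns the avatar toward its combat target and fires a projectile at it.
; It plays a montage from the combat interface's attack list and waits for a tag event to spawn the projectile at the target's location, with optional pitch override.
; Montage, event tag and socket tag come from separate Random calls, so they can differ.
; The ability ends when the montage completes, is interrupted or is cancelled.
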(event `self.K2_ActivateAbility`
  (bind _returnvalue (`self.GetAvatarActorFromActorInfo`))
  (bind _returnvalue_2 (message `AuraEnemyInterface.GetCombatTarget` _returnvalue))
  ; 可以不CAST到combatInterface
  (bind _ascombat_interface (cast `CombatInterface` _returnvalue))
  (bind _returnvalue_3 (`Actor.K2_GetActorLocation` _returnvalue_2))
  (`CombatInterface.UpdateFacingTarget` _ascombat_interface _returnvalue_3)
  (bind _returnvalue_4 (`CombatInterface.GetAttackMontage` _ascombat_interface))
  (bind (_montage _montagetag _combatsockettag) (break `TaggedMontage` (`KismetArrayLibrary.Array_Random` _returnvalue_4)))
  (bind _output_get (set `self.Montage Tag` _montagetag))
  (`AbilityTask_PlayMontageAndWait.CreatePlayMontageAndWaitProxy` "None" _montage 1.0 "None" false
    (:`then`
      (`AbilityTask_WaitGameplayEvent.WaitGameplayEvent` _output_get null
        (:`EventReceived`
          (`self.SpawnProjectile` _returnvalue_3 _combatsockettag (`self.Is Override Pitch`) (`self.Override Pitch`)))))
    (:`OnCompleted`
      (`self.K2_EndAbility` :!label _label))
    (:`OnInterrupted`
      (goto _label))
    (:`OnCancelled`
      (goto _label))))