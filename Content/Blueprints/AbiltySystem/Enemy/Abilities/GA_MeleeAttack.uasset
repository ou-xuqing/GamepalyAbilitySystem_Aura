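; Enemy melee attack gameplay ability: turns the avatar toward its combat target and plays a random attack montage.
; It waits for the montage's tagged gameplay event, then damages non-friendly living actors in a small sphere at that attack's combat socket.
; A hit fires a MeleeImpact gameplay cue carrying the montage tag, location and target.
; The ability ends after the hit check or when the montage completes, is interrupted or is cancelled.
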(event `self.K2_ActivateAbility`
  (bind _returnvalue (`self.GetAvatarActorFromActorInfo`))
  (bind _returnvalue_2 (`self.GetAvatarActorFromActorInfo`))
  (set `self.HasHitTarget` false)
  ; 获得攻击目标的位置，该位置在BTTaskAttack中设置，然后修改朝向
  (bind _returnvalue_3 (message `AuraEnemyInterface.GetCombatTarget` _returnvalue_2))
  (bind _output_get (set `self.CombatTarget` _returnvalue_3))
  (bind _ascombat_interface (cast `CombatInterface` _returnvalue_2))
  (`CombatInterface.UpdateFacingTarget` _ascombat_interface (`Actor.K2_GetActorLocation` _output_get))
  ; 随机选择攻击montage
  (bind _returnvalue_4 (message `CombatInterface.GetAttackMontage` _returnvalue_2))
  (bind _output_get_2 (set `self.AttackMontage` (`KismetArrayLibrary.Array_Random` _returnvalue_4)))
  (bind (_montage _montagetag _combatsockettag) (break `TaggedMontage` _output_get_2))
  ; 攻击可能存在被打断的情况，此时直接结束能力
  (`AbilityTask_PlayMontageAndWait.CreatePlayMontageAndWaitProxy` "None" _montage 1.0 "None" false
    (:`then`
      ;; 等待AN_MontageEvent事件发生
      (`AbilityTask_WaitGameplayEvent.WaitGameplayEvent` _montagetag null
        (:`EventReceived`
          ; 捕获攻击目标后进行伤害计算
          (bind _returnvalue_5 (message `CombatInterface.GetCombatSocketLocation` _returnvalue _combatsockettag))
          (bind _output_get_3 (set `self.CombatSocketLocation` _returnvalue_5))
          (bind _outoverlappingactor (`AuraAbilitySystemLibrary.GetLiversWithinRadius` _returnvalue (`|MakeArray` _returnvalue) 40.0 _output_get_3))
          (for _array_element _outoverlappingactor
            (bind _returnvalue_6 (`AuraAbilitySystemLibrary.IsNotFriend` _returnvalue _array_element))
            (if _returnvalue_6
              (`self.CauseDamage` _array_element)
              (set `self.HasHitTarget` true)))
          (if (`self.HasHitTarget`)
            (`self.K2_ExecuteGameplayCueWithParams` (struct :`TagName` "GameplayCue.MeleeImpact") (`AbilitySystemBlueprintLibrary.MakeGameplayCueParameters` 0.0 0.0 (struct) (struct) (struct) (`BlueprintGameplayTagLibrary.MakeGameplayTagContainerFromTag` (`.MontageTag` (break `TaggedMontage` (`self.AttackMontage`)))) (struct) (`self.CombatSocketLocation`) (0.0 0.0 0.0) null (`self.GetAvatarActorFromActorInfo`) (`self.CombatTarget`)))))))
    (:`OnCompleted`
      _)
    (:`OnInterrupted`
      _)
    (:`OnCancelled`
      _))
  (`self.K2_EndAbility`))