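; BP_EnemyBase is a base enemy character Blueprint that handles spawn scaling, attack facing and dissolve effects.
; On BeginPlay a timeline drives the mesh's uniform scale.
; UpdateFacingTarget feeds a location to Motion Warping's "Facing Target" so attack montages turn toward the player.
; Two dissolve events run separate timelines, one for the weapon, animating the Dissolve scalar on passed-in dynamic material instances.
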(event `self.ReceiveBeginPlay`
  (bind (_direction _sacletrack) (`Timeline|ScaleTimeline`)
    (:`Update`
      (`SceneComponent.SetRelativeScale3D` (`self.Mesh`) (`KismetMathLibrary.MakeVector` _sacletrack _sacletrack _sacletrack)))))

(event `CombatInterface.UpdateFacingTarget`
  (params (TargetLocation :type "Vector Structure (by ref)"))
  ; 使用motionwarp插件，在执行攻击AM时将敌人面向player
  (`MotionWarpingComponent.AddOrUpdateWarpTargetFromLocation` (`self.MotionWarping`) "Facing Target" TargetLocation))

(event `self.StartDissolveTimeline`
  (params (DisMaterialInsDyn :type "MaterialInstanceDynamic Object Reference"))
  (bind (_direction _dissolvetarck) (`Timeline|DissolveTimeline`)
    (:`Update`
      (`MaterialInstanceDynamic.SetScalarParameterValue` DisMaterialInsDyn "Dissolve" _dissolvetarck))))

(event `self.StartWeaponDissolveTimeline`
  (params (DisMaterialInsDyn :type "MaterialInstanceDynamic Object Reference"))
  (bind (_direction _newtrack_0) (`Timeline|WeaponDissolveTimeline`)
    (:`Update`
      (`MaterialInstanceDynamic.SetScalarParameterValue` DisMaterialInsDyn "Dissolve" _newtrack_0))))

(fn `UserConstructionScript`)